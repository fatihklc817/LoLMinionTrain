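; BP_Killer is a trigger volume that destroys minions of its configured team when they enter it.
; Its Box overlap event casts the entering actor to LMTMinionBase and ignores anything else.
; The IsBlueTeam flag selects the target: Blue minions when true, any non-Blue minion when false.
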(event OnComponentBeginOverlap(Box)
  (params (OverlappedComponent :type Primitive%20Component%20Object%20Reference) (OtherActor :type Actor%20Object%20Reference) (OtherComp :type Primitive%20Component%20Object%20Reference) (OtherBodyIndex :type Integer) (bFromSweep :type Boolean) (SweepResult :type Hit%20Result%20Structure%20%28by%20ref%29))
  (bind _aslmtminion_base (Utilities|Casting|CastToLMTMinionBase OtherActor))
  (Variables|Default|SetAs%20LMTMinion%20Base _aslmtminion_base)
  (if (Variables|Default|GetIsBlueTeam)
    (if (Utilities|Enum|Equal(Enum) (Class|LMTBaseCharacter|GetTeam _aslmtminion_base) "Blue")
      (Actor|DestroyActor (Variables|Default|GetAs%20LMTMinion%20Base)))
    (elif (not (Utilities|Enum|Equal(Enum) (Class|LMTBaseCharacter|GetTeam _aslmtminion_base) "Blue"))
      (Actor|DestroyActor (Variables|Default|GetAs%20LMTMinion%20Base)))))

(event EventBeginPlay)

(event Collision|EventActorBeginOverlap
  (params (OtherActor :type Actor%20Object%20Reference)))

(event EventTick
  (params (DeltaSeconds :type Float%20%28single-precision%29)))

(fn ConstructionScript)